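; MoveableCube_BP is a placeable cube that the player can push.
; Two overlap volumes, one for the X axis and one for the Y axis, respond only to Player_BP, setting its IsPusing flag on entry and clearing it on exit.
; Both entering and leaving either volume turn physics simulation on for the cube; the graph never turns it off.
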(event OnComponentBeginOverlap(Y-AxisCollision)
  (params (OverlappedComponent :type Primitive%20Component%20Object%20Reference) (OtherActor :type Actor%20Object%20Reference) (OtherComp :type Primitive%20Component%20Object%20Reference) (OtherBodyIndex :type Integer) (bFromSweep :type Boolean) (SweepResult :type Hit%20Result%20Structure%20%28by%20ref%29))
  ;[1 1 1] Y-Axis Collision
  (bind _asplayer_bp (Utilities|Casting|CastToPlayer_BP OtherActor))
  (Physics|SetSimulatePhysics (Variables|Default|GetCube) true)
  (Variables|/Game/Apocalypse/Core/Characters/Player/Player_BP.Player_BP_C|SetisPusing _asplayer_bp true))

(event OnComponentEndOverlap(Y-AxisCollision)
  (params (OverlappedComponent :type Primitive%20Component%20Object%20Reference) (OtherActor :type Actor%20Object%20Reference) (OtherComp :type Primitive%20Component%20Object%20Reference) (OtherBodyIndex :type Integer))
  ;[1 1 1] Y-Axis Collision
  (bind _asplayer_bp (Utilities|Casting|CastToPlayer_BP OtherActor))
  (Physics|SetSimulatePhysics (Variables|Default|GetCube) true)
  (Variables|/Game/Apocalypse/Core/Characters/Player/Player_BP.Player_BP_C|SetisPusing _asplayer_bp false))

(event OnComponentBeginOverlap(X-AxisCollision)
  (params (OverlappedComponent :type Primitive%20Component%20Object%20Reference) (OtherActor :type Actor%20Object%20Reference) (OtherComp :type Primitive%20Component%20Object%20Reference) (OtherBodyIndex :type Integer) (bFromSweep :type Boolean) (SweepResult :type Hit%20Result%20Structure%20%28by%20ref%29))
  (bind _asplayer_bp (Utilities|Casting|CastToPlayer_BP OtherActor))
  (Physics|SetSimulatePhysics (Variables|Default|GetCube) true)
  (Variables|/Game/Apocalypse/Core/Characters/Player/Player_BP.Player_BP_C|SetisPusing _asplayer_bp true))

(event OnComponentEndOverlap(X-AxisCollision)
  (params (OverlappedComponent :type Primitive%20Component%20Object%20Reference) (OtherActor :type Actor%20Object%20Reference) (OtherComp :type Primitive%20Component%20Object%20Reference) (OtherBodyIndex :type Integer))
  (bind _asplayer_bp (Utilities|Casting|CastToPlayer_BP OtherActor))
  (Physics|SetSimulatePhysics (Variables|Default|GetCube) true)
  (Variables|/Game/Apocalypse/Core/Characters/Player/Player_BP.Player_BP_C|SetisPusing _asplayer_bp false))

(fn ConstructionScript)