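; Player character Blueprint that turns player input into basic movement and camera control.
; Axis inputs move the character along its forward and right vectors and feed controller yaw and pitch for looking.
; Jump and crouch follow press and release through the built-in Character functions, while holding Sprint swaps max walk speed to RunSpeed and release restores a hardcoded default.
; BeginPlay, Tick, overlap and the construction script are empty.
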(event EventBeginPlay)

(event Collision|EventActorBeginOverlap
  (params (OtherActor :type Actor%20Object%20Reference)))

(event EventTick
  (params (DeltaSeconds :type Float%20%28single-precision%29)))

(event Input|ActionEvents|InputActionJump
  (params (Key :type Key%20Structure :default "None"))
  ;[0.2917 0.1303 1] Jump (Spacebar)
  (:Pressed
    (Character|Jump))
  (:Released
    (Character|StopJumping)))

(event Input|ActionEvents|InputActionSprint
  (params (Key :type Key%20Structure :default "None"))
  ;[0.7587 0 1] Sprint (LeftShift)
  (:Pressed
    (Variables|/Script/Engine.CharacterMovementComponent|SetMaxWalkSpeed (Variables|Character|GetCharacterMovement) (Variables|Default|GetRun_Speed)))
  (:Released
    (Variables|/Script/Engine.CharacterMovementComponent|SetMaxWalkSpeed (Variables|Character|GetCharacterMovement) 6e+02)))

(event Input|ActionEvents|InputActionCrouch
  (params (Key :type Key%20Structure :default "None"))
  ;[0 0.07684 0.1562] Crouch (LeftCtrl)
  (:Pressed
    (Character|Crouch))
  (:Released
    (Character|UnCrouch)))

(event Input|AxisEvents|InputAxisForward_Backwards
  (params (AxisValue :type Float%20%28single-precision%29))
  ;[0 0.7224 1] Movement values for character (WASD)
  (Pawn|Input|AddMovementInput (Transformation|GetActorForwardVector) AxisValue false))

(event Input|AxisEvents|InputAxisLeft_Right
  (params (AxisValue :type Float%20%28single-precision%29))
  ;[0 0.7224 1] Movement values for character (WASD)
  (Pawn|Input|AddMovementInput (Transformation|GetActorRightVector) AxisValue false))

(event Input|AxisEvents|InputAxisLook_Left_Right
  (params (AxisValue :type Float%20%28single-precision%29))
  ;[0 1 0.7583] Camera values for character
  (Pawn|Input|AddControllerYawInput AxisValue))

(event Input|AxisEvents|InputAxisLook_Up_Down
  (params (AxisValue :type Float%20%28single-precision%29))
  ;[0 1 0.7583] Camera values for character
  (Pawn|Input|AddControllerPitchInput AxisValue))

(fn ConstructionScript)